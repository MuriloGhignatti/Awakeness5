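; BP_Pickup is a physics-simulated world pickup for an inventory item.
; The construction script sets the mesh from the Item class's default ItemInfo and takes sizing from those defaults or per-instance overrides, according to UseDefaults.
; It dynamically adds a box, sphere or capsule, chosen by Collision, attached to the mesh.
; Overlaps route to BeginOverlap, which only prints whether the actor is a ThirdPersonCharacter; no collection logic exists.
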(event `self.BoxCollision.OnComponentBeginOverlap`
  (params (OverlappedComponent :type "PrimitiveComponent Object Reference") (OtherActor :type "Actor Object Reference") (OtherComp :type "PrimitiveComponent Object Reference") (OtherBodyIndex :type Integer) (bFromSweep :type Boolean) (SweepResult :type "HitResult Structure (by ref)"))
  (`self.BeginOverlap` OtherActor))

(event `self.SphereCollision.OnComponentBeginOverlap`
  (params (OverlappedComponent :type "PrimitiveComponent Object Reference") (OtherActor :type "Actor Object Reference") (OtherComp :type "PrimitiveComponent Object Reference") (OtherBodyIndex :type Integer) (bFromSweep :type Boolean) (SweepResult :type "HitResult Structure (by ref)"))
  (`self.BeginOverlap` OtherActor))

(event `self.CapsuleCollision.OnComponentBeginOverlap`
  (params (OverlappedComponent :type "PrimitiveComponent Object Reference") (OtherActor :type "Actor Object Reference") (OtherComp :type "PrimitiveComponent Object Reference") (OtherBodyIndex :type Integer) (bFromSweep :type Boolean) (SweepResult :type "HitResult Structure (by ref)"))
  (`self.BeginOverlap` OtherActor))

(fn `BeginOverlap`
  (params (OtherActor :type "Actor Object Reference (by ref)"))
  (cast `/Game/ThirdPersonCPP/Blueprints/ThirdPersonCharacter` OtherActor
    (:`then`
      (`KismetSystemLibrary.PrintString` "Yas"))
    (:`CastFailed`
      (`KismetSystemLibrary.PrintString` "No"))))

(fn `UserConstructionScript`
  (locals (defaultMeshScale :type "Vector Structure") (defaultBoxCollisionScale :type "Vector Structure") (defaultRadius :type "Float (double-precision)") (defaultHalfReight :type "Float (double-precision)") (defaultMeshPosition :type "Vector Structure") (defaultWeight :type "Float (double-precision)") (localItemMesh :type "StaticMesh Object Reference"))
  (bind (_id _iteminfo) (defaults `Object` (`self.Item`)))
  (set `local.defaultWeight` (`.Weight` (break `ItemInfo` _iteminfo)))
  (set `local.localItemMesh` (`.PickupMesh` (break `ItemInfo` _iteminfo)))
  (set `local.defaultMeshScale` (`.MeshScale` (break `ItemInfo` _iteminfo)))
  (set `local.defaultMeshPosition` (`.MeshPosition` (break `ItemInfo` _iteminfo)))
  (set `local.defaultBoxCollisionScale` (`.BoxCollisionScale` (break `ItemInfo` _iteminfo)))
  (set `local.defaultRadius` (`.Radius` (break `ItemInfo` _iteminfo)))
  (set `local.defaultHalfReight` (`.HalfHeight` (break `ItemInfo` _iteminfo)))
  (`PrimitiveComponent.SetCollisionEnabled` (`self.ItemMesh`) "QueryAndPhysics")
  (`PrimitiveComponent.SetSimulatePhysics` (`self.ItemMesh`) true)
  (`StaticMeshComponent.SetStaticMesh` (`self.ItemMesh`) (`local.localItemMesh`))
  (if (`self.UseDefaults`)
    (`SceneComponent.SetRelativeScale3D` (`self.ItemMesh`) (`local.defaultMeshScale`))
    (`SceneComponent.K2_SetRelativeLocation` (`self.ItemMesh`) (`local.defaultMeshPosition`) false false)
    (else
      (`SceneComponent.SetRelativeScale3D` (`self.ItemMesh`) (`self.Mesh Scale`))
      (`SceneComponent.K2_SetRelativeLocation` (`self.ItemMesh`) (`self.Mesh Position`) false false)))
  (switch `/Game/InventorySystem/Blueprints/E_Collision` (`self.Collision`)
    (:`NewEnumerator0`
      (bind _returnvalue (`AddComponent|NODE_AddBoxComponent-0`))
      (set `self.BoxCollision` _returnvalue)
      (if (`self.UseDefaults`)
        (`SceneComponent.SetRelativeScale3D` (`self.BoxCollision`) (`local.defaultBoxCollisionScale`))
        (else
          (`SceneComponent.SetRelativeScale3D` (`self.BoxCollision`) (`self.Box Collision Scale`))))
      (`SceneComponent.K2_AttachToComponent` (`self.BoxCollision`) (`self.ItemMesh`) "None" "KeepRelative" "KeepRelative" "KeepRelative" true)
      (`PrimitiveComponent.SetCollisionEnabled` (`self.BoxCollision`) "QueryAndPhysics")
      (`PrimitiveComponent.SetSimulatePhysics` (`self.BoxCollision`) true))
    (:`NewEnumerator1`
      (bind _returnvalue_2 (`AddComponent|NODE_AddSphereComponent-0`))
      (set `self.SphereCollision` _returnvalue_2)
      (if (`self.UseDefaults`)
        (`SphereComponent.SetSphereRadius` (`self.SphereCollision`) (`local.defaultRadius`) true)
        (else
          (`SphereComponent.SetSphereRadius` (`self.SphereCollision`) (`self.Radius`) true)))
      (`SceneComponent.K2_AttachToComponent` (`self.SphereCollision`) (`self.ItemMesh`) "None" "KeepRelative" "KeepRelative" "KeepRelative" true)
      (`PrimitiveComponent.SetCollisionEnabled` (`self.SphereCollision`) "QueryAndPhysics")
      (`PrimitiveComponent.SetSimulatePhysics` (`self.SphereCollision`) true))
    (:`NewEnumerator2`
      (bind _returnvalue_3 (`AddComponent|NODE_AddCapsuleComponent-0`))
      (set `self.CapsuleCollision` _returnvalue_3)
      (if (`self.UseDefaults`)
        (`CapsuleComponent.SetCapsuleRadius` (`self.CapsuleCollision`) (`local.defaultRadius`) true)
        (`CapsuleComponent.SetCapsuleHalfHeight` (`self.CapsuleCollision`) (`local.defaultHalfReight`) true)
        (else
          (`CapsuleComponent.SetCapsuleRadius` (`self.CapsuleCollision`) (`self.Radius`) true)
          (`CapsuleComponent.SetCapsuleHalfHeight` (`self.CapsuleCollision`) (`self.Half Height`) true)
          (`SceneComponent.K2_SetRelativeRotation` (`self.CapsuleCollision`) (`self.Rotation`) false false)))
      (`SceneComponent.K2_AttachToComponent` (`self.CapsuleCollision`) (`self.ItemMesh`) "None" "KeepRelative" "KeepRelative" "KeepRelative" true)
      (`PrimitiveComponent.SetCollisionEnabled` (`self.CapsuleCollision`) "QueryAndPhysics")
      (`PrimitiveComponent.SetSimulatePhysics` (`self.CapsuleCollision`) true))))